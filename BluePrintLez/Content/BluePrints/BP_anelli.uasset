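; BP_anelli is a decorative ring actor with a Sphere and a Torus that spins slowly during play.
; The construction script gives each mesh a dynamic instance of the Ball_ring material with its own Emission value, then applies a shared random-hue Color to both.
; Tick adds a small fixed local rotation each frame, unscaled by delta time, so spin speed follows frame rate.
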(event `self.ReceiveTick`
  (params (DeltaSeconds :type "Float (single-precision)"))
  (`self.K2_AddActorLocalRotation` (struct :`Yaw` 0.2)))

(fn `UserConstructionScript`
  (bind _torus (`self.Torus`))
  (bind _color (`self.Color`))
  (`PrimitiveComponent.CreateDynamicMaterialInstance` (`self.Sphere`) 0 "/Game/textures_mat/ball_ring.ball_ring" "MI_sphere")
  (`PrimitiveComponent.CreateDynamicMaterialInstance` (`self.Torus`) 0 "/Game/textures_mat/ball_ring.ball_ring" "MI_torus")
  (`MeshComponent.SetScalarParameterValueOnMaterials` (`self.Sphere`) "Emission" (`self.SphereEmission`))
  (`MeshComponent.SetScalarParameterValueOnMaterials` _torus "Emission" (`self.TorusEmission`))
  (`KismetMathLibrary.LinearColor_SetRandomHue` _color)
  (`MeshComponent.SetColorParameterValueOnMaterials` _torus "Color" _color)
  (`MeshComponent.SetColorParameterValueOnMaterials` (`self.Sphere`) "Color" _color))