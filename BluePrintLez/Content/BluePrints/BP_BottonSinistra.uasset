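; BP_BottonSinistra is a trigger button that makes matching BP_Tubo pipes rotate left while the BP_pg character stands in its sphere.
; At BeginPlay it caches every BP_Tubo actor in the level.
; Sphere begin overlap calls RuotaSinistra on pipes whose TagTubo matches the button's Tag.
; End overlap calls FermaSinistra on all cached pipes, regardless of tag.
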(event `self.ReceiveBeginPlay`
  (bind _outactors (`GameplayStatics.GetAllActorsOfClass` "/Game/BluePrints/BP_Tubo.BP_Tubo_C"))
  (set `self.Tubi` _outactors))

(event `self.Sphere.OnComponentBeginOverlap`
  (params (OverlappedComponent :type "PrimitiveComponent Object Reference") (OtherActor :type "Actor Object Reference") (OtherComp :type "PrimitiveComponent Object Reference") (OtherBodyIndex :type Integer) (bFromSweep :type Boolean) (SweepResult :type "HitResult Structure (by ref)"))
  (cast `/Game/PG/BP_pg` OtherActor)
  (for _array_element (`self.Tubi`)
    (if (== (`/Game/BluePrints/BP_Tubo.TagTubo` _array_element) (`self.Tag`))
      (`/Game/BluePrints/BP_Tubo.Ruota Sinistra` _array_element))))

(event `self.Sphere.OnComponentEndOverlap`
  (params (OverlappedComponent :type "PrimitiveComponent Object Reference") (OtherActor :type "Actor Object Reference") (OtherComp :type "PrimitiveComponent Object Reference") (OtherBodyIndex :type Integer))
  (cast `/Game/PG/BP_pg` OtherActor)
  (for _array_element (`self.Tubi`)
    (`/Game/BluePrints/BP_Tubo.FermaSinistra` _array_element)))

(fn `ReceiveActorBeginOverlap`
  (params (OtherActor :type "Actor Object Reference")))

(fn `UserConstructionScript`)