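; BP_checkPoint is a checkpoint platform that sets the player's respawn point in the kill zone actor, BP_killatore, found on BeginPlay.
; The first time BP_pg overlaps its box, it writes the cube's location plus a vertical offset to the kill zone's checkpoint position.
; It then plays a sound and raises the cube's emission through a timeline.
; The construction script gives each instance a dynamic material with configurable color and emission.
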(event `self.ReceiveBeginPlay`
  ; Referencing the kill zone
  (bind _returnvalue (`GameplayStatics.GetActorOfClass` "/Game/BluePrints/BP_killatore.BP_killatore_C"))
  (set `self.reference` _returnvalue))

(event `self.Box.OnComponentBeginOverlap`
  (params (OverlappedComponent :type "PrimitiveComponent Object Reference") (OtherActor :type "Actor Object Reference") (OtherComp :type "PrimitiveComponent Object Reference") (OtherBodyIndex :type Integer) (bFromSweep :type Boolean) (SweepResult :type "HitResult Structure (by ref)"))
  (bind _returnvalue (`SceneComponent.K2_GetComponentLocation` (`self.Cube`)))
  ; Check the collision
  (if (== (`GameplayStatics.GetObjectClass` OtherActor) "/Game/PG/BP_pg.BP_pg_C")
    ; Checking if the player has already reached this checkpoint
    (if (not (`self.IsReached`))
      (set `self.IsReached` true)
      ; Setting the respawn position to the center of the platform + offset
      (set `/Game/BluePrints/BP_killatore.CheckpointPosition` (+ (`KismetMathLibrary.MakeVector` 0.0 0.0 (`self.RespawnOffset`)) _returnvalue) (`self.reference`))
      ; Audio clip player
      (`GameplayStatics.PlaySoundAtLocation` "/Game/Audio/AC_cassiera.AC_cassiera" _returnvalue (struct) 0.5 1.0 0.0 null null null null)
      ; Checkpoint reached - emission animation
      (bind (_direction _lerp_alpha) (`Timeline|CheckpointReachedTimeline`)
        (:`Update`
          (`MeshComponent.SetScalarParameterValueOnMaterials` (`self.Cube`) "Emission" (`KismetMathLibrary.Lerp` 0.0 0.2 _lerp_alpha)))))))

(fn `UserConstructionScript`
  ; MI for this particular object. Color and emissiopn can be changed
  (bind _returnvalue (`KismetMaterialLibrary.CreateDynamicMaterialInstance` "/Game/textures_mat/mat_base.mat_base" "Minstance"))
  (`PrimitiveComponent.SetMaterial` (`self.Cube`) 0 _returnvalue)
  (`MaterialInstanceDynamic.SetVectorParameterValue` _returnvalue "Color" (`self.ColorValue`))
  (`MaterialInstanceDynamic.SetScalarParameterValue` _returnvalue "Emission" (`self.EmissionValue`)))