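; BP_Rotatoria is an actor with a Cylinder that spins continuously around its yaw axis and has a configurable color and glow.
; The construction script creates a dynamic instance of Mat_base on the cylinder and feeds ColorValue and EmissionValue into its Color and Emission parameters.
; Tick adds DeltaRotation as relative yaw each frame without delta-time scaling, so spin speed depends on frame rate.
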(event `self.ReceiveTick`
  (params (DeltaSeconds :type "Float (single-precision)"))
  (`SceneComponent.K2_AddRelativeRotation` (`self.Cylinder`) (`KismetMathLibrary.MakeRotator` 0.0 0.0 (`self.DeltaRotation`)) false false))

(fn `UserConstructionScript`
  ; MI for this particular object. Color and emissiopn can be changed
  (bind _returnvalue (`KismetMaterialLibrary.CreateDynamicMaterialInstance` "/Game/textures_mat/mat_base.mat_base" "Minstance"))
  (`PrimitiveComponent.SetMaterial` (`self.Cylinder`) 0 _returnvalue)
  (`MaterialInstanceDynamic.SetVectorParameterValue` _returnvalue "Color" (`self.ColorValue`))
  (`MaterialInstanceDynamic.SetScalarParameterValue` _returnvalue "Emission" (`self.EmissionValue`)))