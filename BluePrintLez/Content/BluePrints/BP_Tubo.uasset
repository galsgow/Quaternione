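; BP_Tubo is a tube actor whose mesh can be rotated left or right through external start and stop events.
; Each direction has a timeline used as an update loop, adding its own fixed local rotation every update, so speed depends on frame rate.
; The construction script creates a dynamic material instance from Mat_base, exposing per-object color and emission.
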(event `self.ReceiveBeginPlay`)

(event `Ruota Sinistra`
  (`Timeline|TimelineSinistra` :!label _label
    (:`Update`
      (`SceneComponent.K2_AddLocalRotation` (`self.CubeGridToolOutput_D5A149CE`) (`self.VelocitàSinistra`) false false))))

(event `FermaSinistra`
  (goto _label :!via `Stop`))

(event `RuotaDestra`
  (`Timeline|TimelineDestra` :!label _label_2
    (:`Update`
      (`SceneComponent.K2_AddLocalRotation` (`self.CubeGridToolOutput_D5A149CE`) (`self.VelocitàDestra`) false false))))

(event `FermaDestra`
  (goto _label_2 :!via `Stop`))

(fn `UserConstructionScript`
  ; MI for this particular object. Color and emissiopn can be changed
  (bind _returnvalue (`KismetMaterialLibrary.CreateDynamicMaterialInstance` "/Game/textures_mat/mat_base.mat_base" "Minstance"))
  (`PrimitiveComponent.SetMaterial` (`self.CubeGridToolOutput_D5A149CE`) 0 _returnvalue)
  (`MaterialInstanceDynamic.SetVectorParameterValue` _returnvalue "Color" (`self.ColorValue`))
  (`MaterialInstanceDynamic.SetScalarParameterValue` _returnvalue "Emission" (`self.EmissionValue`)))